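; DataLoaderActor loads a sectioned text config file at BeginPlay or on L release, creating it from a template if it cannot be read.
; Its line parser strips comments, runs console commands, rebinds action and axis mappings, then rebuilds keymaps.
; Variables are set by reflection on itself or tag-selected actors, with multiline quoted strings accumulated.
; It then fires a finished callback and notifies all DataLoaderInterface actors.
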(event EventBeginPlay
  (Development|PrintString "Preload")
  (Utilities|FlowControl|Delay 1.0)
  (CallFunction|LoadDatafromFile)
  (Development|PrintString "PostLoad"))

(event Input|ActionEvents|InputActionInteractionPickup
  (params (Key :type Key%20Structure))
  (:Pressed
    (Development|PrintString "InteractionPickup Pressed" true false))
  (:Released
    (Development|PrintString "InteractionPickup  Released" true false)))

(event Input|AxisEvents|InputAxisMoveTest
  (params (AxisValue :type Float%20%28single-precision%29))
  (if (> (Math|Float|Absolute(Float) AxisValue) 0.0)
    (Development|PrintString (Utilities|String|Append "Move  Test Axis : " (Utilities|String|ToString(Float) AxisValue)) true false "(R=0.000000,G=0.660000,B=1.000000,A=1.000000)" 0.0)))

(event Input|KeyboardEvents|L
  (params (Key :type Key%20Structure))
  (:Released
    (CallFunction|LoadDatafromFile)
    (Development|PrintString "PostLoad")))

(fn ConstructionScript)

(fn DecodeandExecuteContentsOfFile
  (params (FileNameWithFullPath :type String))
  (LocalVariables|SetInFilePath FileNameWithFullPath)
  (if (.ReturnValue (Class|FileSDKBPLibrary|ReadLinesfromFile (LocalVariables|GetInFilePath) "/Script/FileSDK.FileSDKLineReader"))
    (LocalVariables|SetAllLinesInTheFile (.Lines (Class|FileSDKBPLibrary|ReadLinesfromFile (LocalVariables|GetInFilePath) "/Script/FileSDK.FileSDKLineReader")))
    (for (_array_element _array_index) (LocalVariables|GetAllLinesInTheFile)
      (LocalVariables|SetCurrentLine _array_element)
      (LocalVariables|SetCurrentLineNumber _array_index)
      ;[1 1 1] If accumulating multiline string,
      ; Continue accumulation
      (if (LocalVariables|GetbShouldAccumulateString?)
        ;[1 1 1] Single and Multiline Strings accumulation on setup
        (LocalVariables|SetValue (LocalVariables|GetCurrentLine))
        ;;[1 1 1] Accumulated string has start quote " ?
        (if (Utilities|String|Contains (LocalVariables|GetAccumulatedString) "\"") :!label _label
          (if (> (Utilities|String|FindSubstring (LocalVariables|GetValue) "\"" false true) -1)
            ;;[1 1 1] End Accumulation
            (LocalVariables|SetValue (Utilities|String|GetSubstring (LocalVariables|GetValue) 0 (+ (Utilities|String|FindSubstring (LocalVariables|GetValue) "\"" false true) 1)) :!label _label_2)
            (LocalVariables|SetAccumulatedString (Utilities|String|Append (LocalVariables|GetAccumulatedString) (LocalVariables|GetValue)))
            (LocalVariables|SetbShouldAccumulateString? false)
            ;;[1 1 1] Remove characters after end quote
            (LocalVariables|SetAccumulatedString (Utilities|String|LeftChop (LocalVariables|GetAccumulatedString) (select (> (Utilities|String|FindSubstring (LocalVariables|GetAccumulatedString) "\"" false true) -1) (- (Utilities|String|Len (LocalVariables|GetAccumulatedString)) (Utilities|String|FindSubstring (LocalVariables|GetAccumulatedString) "\"" false true)) 0)))
            ;;[1 1 1] Remove characters before start quote
            (LocalVariables|SetAccumulatedString (Utilities|String|RightChop (LocalVariables|GetAccumulatedString) (+ (Utilities|String|FindSubstring (LocalVariables|GetAccumulatedString) "\"") 1)))
            (CallFunction|UpdatePropertyonTargetObject (LocalVariables|GetTargetObjects) (LocalVariables|GetNameOfThePropertyToUdpateAfterAcumulation) (LocalVariables|GetAccumulatedString))
            (else
              ;;[1 1 1] Start/ Continue accumulation
              (LocalVariables|SetAccumulatedString (Utilities|String|Append (LocalVariables|GetAccumulatedString) (LocalVariables|GetValue)) :!label _label_3)
              (LocalVariables|SetAccumulatedString (Utilities|String|Append (LocalVariables|GetAccumulatedString) " 
"))))
          (else
            ;;[1 1 1] Has 2 or more " quotes in current line?
            (if (and (!= (Utilities|String|FindSubstring (LocalVariables|GetValue) "\"") (Utilities|String|FindSubstring (LocalVariables|GetValue) "\"" false true)) (> (Utilities|String|FindSubstring (LocalVariables|GetValue) "\"" false true) -1))
              (goto _label_2)
              (else
                (goto _label_3)))))
        (else
          ;[1 1 1] Ignore comments
          (if (or (> (Utilities|String|FindSubstring (LocalVariables|GetCurrentLine) "#") -1) (> (Utilities|String|FindSubstring (LocalVariables|GetCurrentLine) "//") -1))
            (LocalVariables|SetCurrentLine (Utilities|String|LeftChop (LocalVariables|GetCurrentLine) (- (Utilities|String|Len (LocalVariables|GetCurrentLine)) (select (and (> (Utilities|String|FindSubstring (LocalVariables|GetCurrentLine) "#") -1) (> (Utilities|String|FindSubstring (LocalVariables|GetCurrentLine) "//") -1)) (Math|Integer|Min(Integer) (Utilities|String|FindSubstring (LocalVariables|GetCurrentLine) "#") (Utilities|String|FindSubstring (LocalVariables|GetCurrentLine) "//")) (Math|Integer|Max(Integer) (Utilities|String|FindSubstring (LocalVariables|GetCurrentLine) "#") (Utilities|String|FindSubstring (LocalVariables|GetCurrentLine) "//")))))))
          ;[1 1 1] Ignore 0 length lines
          (if (> (Utilities|String|Len (Utilities|String|TrimTrailing (Utilities|String|Trim (LocalVariables|GetCurrentLine)))) 0)
            (LocalVariables|SetCurrentLine (Utilities|String|TrimTrailing (Utilities|String|Trim (LocalVariables|GetCurrentLine))))
            ;[1 1 1] Set, find and update section tags
            (if (and (Utilities|String|StartsWith (LocalVariables|GetCurrentLine) "[") (Utilities|String|EndsWith (LocalVariables|GetCurrentLine) "]"))
              (bind _output_get (LocalVariables|SetCurrentSection (Utilities|String|Replace (LocalVariables|GetCurrentLine) " ")))
              (Utilities|Set|Add (LocalVariables|GetAllSectionsFoundInTheFile) _output_get)
              (else
                (switch string (LocalVariables|GetCurrentSection)
                  (:Default
                    (Development|PrintString (Utilities|String|Append "DataLoaderActor: DecodeFile : Undefined Section in:   " (LocalVariables|GetInFilePath) "   at  Line :  " (Utilities|String|ToString(Integer) (+ (LocalVariables|GetCurrentLineNumber) 1))) true true "(R=1.000000,G=0.000000,B=0.012401,A=1.000000)"))
                  (:[ConsoleCommands]
                    (Development|ExecuteConsoleCommand (LocalVariables|GetCurrentLine) 0))
                  (:[InputActionMappings]
                    (CallFunction|AddNewActionMappingfromLine (LocalVariables|GetCurrentLine)))
                  (:[InputAxisMappings]
                    (CallFunction|AddNewAxisMapping (LocalVariables|GetCurrentLine)))
                  (:[Variables]
                    ;[1 1 1] Test Variables
                    (LocalVariables|SetKey (.Key (CallFunction|GetKeyandValue (LocalVariables|GetCurrentLine))))
                    (LocalVariables|SetValue (.Value (CallFunction|GetKeyandValue (LocalVariables|GetCurrentLine))))
                    (bind _returnvalue (Class|ExposeRuntimeFunctionsBPLibrary|GetFPropertyClassName (CallFunction|GetDefaultObject (LocalVariables|GetTargetObjects)) (Utilities|String|StringToName (LocalVariables|GetKey))))
                    (if (Utilities|Enum|NotEqual(Enum) _returnvalue "StrProperty")
                      (Utilities|FlowControl|Sequence
                        (:then_0
                          ;;[1 1 1] If not string , assign value directly
                          ;;;[1 1 1] Always update tag related properties on this object only
                          (if (or (Utilities|Enum|Equal(Enum) (LocalVariables|GetKey) "TargetObjectTag") (Utilities|Enum|Equal(Enum) (LocalVariables|GetKey) "bEnableSupportForTaggedObjects"))
                            (Class|ExposeRuntimeFunctionsBPLibrary|SetFPropertybyName self (Utilities|String|StringToName (LocalVariables|GetKey)) (LocalVariables|GetValue))
                            (else
                              (CallFunction|UpdatePropertyonTargetObject (LocalVariables|GetTargetObjects) (Utilities|String|StringToName (LocalVariables|GetKey)) (LocalVariables|GetValue)))))
                        (:then_1
                          ;;[1 1 1] if TagetObjectTag is Updated,
                          ;; Update target objects
                          (if (Utilities|Enum|Equal(Enum) (LocalVariables|GetKey) "TargetObjectTag")
                            (if (Variables|Default|GetbEnableSupportForTaggedObjects)
                              (bind _outactors (Actor|GetAllActorswithTag (Variables|Default|GetTargetObjectTag)))
                              (LocalVariables|SetTargetObjects _outactors)))))
                      (else
                        ;[1 1 1] If string, start multiline processing,
                        ; Pre Accumulation setup for multiline string input
                        (LocalVariables|SetNameOfThePropertyToUdpateAfterAcumulation (Utilities|String|StringToName (LocalVariables|GetKey)))
                        (LocalVariables|SetAccumulatedString "")
                        (LocalVariables|SetbShouldAccumulateString? true)
                        (goto _label)))))))))))
    (Utilities|FlowControl|Sequence
      (:then_0
        ;[1 1 1] File decoding completed
        ; Rebuild keymaps if necessory
        (if (or (Utilities|Set|Contains (LocalVariables|GetAllSectionsFoundInTheFile) "[InputAxisMappings]") (Utilities|Set|Contains (LocalVariables|GetAllSectionsFoundInTheFile) "[InputActionMappings]"))
          (Class|InputSettings|ForceRebuildKeymaps (Class|InputSettings|GetInputSettings))))
      (:then_1
        ;[1 1 1] For debugging only
        (Development|PrintString (Utilities|String|Append (Variables|Default|Gets1) " 
------- S2 ------------- 
" (Variables|Default|Gets2) " 
------- S3 ------------- 
" (Variables|Default|Gets3) " 
----------------------"))))
    (else
      ;[1 1 1] Couldnt find file
      (Development|PrintString "DataLoaderActor: Decode and Execute Contents Of File : Cant read File" true true "(R=1.000000,G=0.000000,B=0.012401,A=1.000000)"))))

(fn LoadDatafromFile
  (LocalVariables|SetFileNameWithPath (Utilities|String|Append (Class|KismetSystemLibrary|GetProjectDirectory) (Variables|Default|GetDirectoryName) "/" (Variables|Default|GetFileName)))
  (if (.ReturnValue (Class|FileSDKBPLibrary|ReadStringfromFile (LocalVariables|GetFileNameWithPath)))
    _
    (else
      ;[1 1 1] If file doesn't exist, Create new one from template, at the same location
      (Development|PrintString (Utilities|String|Append (Utilities|GetDisplayName self) " : Couldn't find specified file, creating a new one from template at: 
" (LocalVariables|GetFileNameWithPath)) true true "(R=1.000000,G=0.000000,B=0.086574,A=1.000000)")
      (Class|FileSDKBPLibrary|CreateFile (LocalVariables|GetFileNameWithPath) false true)
      (Class|FileSDKBPLibrary|WriteStringtoFile (LocalVariables|GetFileNameWithPath) (Variables|Default|GetTemplateFileContent) false "AutoDetect")))
  ;[1 1 1] If file exists load data, and call OnDataLoad
  (CallFunction|DecodeandExecuteContentsOfFile (LocalVariables|GetFileNameWithPath))
  ;[1 1 1] Post data load callback
  (Default|CallPostDataLoadingFinished)
  (bind _outactors (Actor|GetAllActorswithInterface "/Game/Blueprints/DataLoader/DataLoaderInterface.DataLoaderInterface_C"))
  (for _array_element _outactors
    (Class|DataLoaderInterface|PostDataLoadCallback(Message) _array_element self)))

(fn GetKeyandValue
  (params (SourceString :type String))
  (bind (_lefts _rights _returnvalue) (Utilities|String|Split SourceString "="))
  ;[1 1 1] Check variable assignment
  (if _returnvalue
    (return (Utilities|String|TrimTrailing (Utilities|String|Trim _lefts)) (Utilities|String|Replace (Utilities|String|Replace (Utilities|String|TrimTrailing (Utilities|String|Trim _rights)) "{") "}"))))

(fn AddNewActionMappingfromLine
  (params (SourceString :type String))
  (bind (_key _value) (CallFunction|GetKeyandValue SourceString))
  ;[1 1 1] Input Action Mappings
  (LocalVariables|SetKey _key)
  (LocalVariables|SetValue _value)
  ;;[1 1 1] Clear old mappings
  (LocalVariables|SetTempActionMappings (Class|InputSettings|GetActionMappingbyName (Class|InputSettings|GetInputSettings) (Utilities|String|StringToName (LocalVariables|GetKey))))
  (for _array_element (LocalVariables|GetTempActionMappings)
    (Class|InputSettings|RemoveActionMapping (Class|InputSettings|GetInputSettings) _array_element false))
  ;[1 1 1] Add new action mappings
  (for _array_element_2 (Utilities|String|ParseIntoArray (LocalVariables|GetValue) ", ")
    (Class|InputSettings|AddActionMapping (Class|InputSettings|GetInputSettings) (Utilities|Struct|MakeInputActionKeyMapping (Utilities|String|StringToName (LocalVariables|GetKey)) (Class|ExposeRuntimeFunctionsBPLibrary|GetKeyfromName (Utilities|String|StringToName (Utilities|String|TrimTrailing (Utilities|String|Trim _array_element_2))))) false)))

(fn AddNewAxisMapping
  (params (SourceString :type String))
  (bind (_key _value) (CallFunction|GetKeyandValue SourceString))
  ;[1 1 1] Input Axis Mappings
  (LocalVariables|SetKey _key)
  (LocalVariables|SetValue _value)
  (LocalVariables|SetTempAxisMappings (Class|InputSettings|GetAxisMappingbyName (Class|InputSettings|GetInputSettings) (Utilities|String|StringToName (LocalVariables|GetKey))))
  (for _array_element (LocalVariables|GetTempAxisMappings)
    (Class|InputSettings|RemoveAxisMapping (Class|InputSettings|GetInputSettings) _array_element false))
  ;[1 1 1] Add new axis mappings
  (for _array_element_2 (Utilities|String|ParseIntoArray (LocalVariables|GetValue) ", ")
    (if (.ReturnValue (Utilities|String|Split _array_element_2 ":"))
      (Class|InputSettings|AddAxisMapping (Class|InputSettings|GetInputSettings) (Utilities|Struct|MakeInputAxisKeyMapping (Utilities|String|StringToName (LocalVariables|GetKey)) (Math|Conversions|ToFloat(Integer) (Utilities|String|TrimTrailing (Utilities|String|Trim (.RightS (Utilities|String|Split _array_element_2 ":"))))) (Class|ExposeRuntimeFunctionsBPLibrary|GetKeyfromName (Utilities|String|StringToName (Utilities|String|TrimTrailing (Utilities|String|Trim (.LeftS (Utilities|String|Split _array_element_2 ":"))))))) false))))

(fn StringtoBool
  (params (Selection :type String))
  (switch string Selection
    (:Default
      (return false))
    (:True
      (return true))
    (:False
      (return false))))

(fn StringtoColor
  (params (SourceString :type String))
  (bind _returnvalue (Utilities|String|ParseIntoArray SourceString "," false))
  (return (Math|Conversions|ToColor(LinearColor) (Utilities|Struct|MakeLinearColor (Math|Conversions|ToFloat(Integer) (Utilities|Array|Get(acopy) _returnvalue)) (Math|Conversions|ToFloat(Integer) (Utilities|Array|Get(acopy) _returnvalue 1)) (Math|Conversions|ToFloat(Integer) (Utilities|Array|Get(acopy) _returnvalue 2)) (Math|Conversions|ToFloat(Integer) (Utilities|Array|Get(acopy) _returnvalue 3))))))

(fn StringtoFloatArray
  (params (TargetArray :type Array%20of%20Floats%20%28single-precision%29) (SourceString :type String))
  (Utilities|Array|Clear TargetArray)
  (for (_array_element _array_index) (Utilities|String|ParseIntoArray SourceString ",")
    (Utilities|Array|SetArrayElem TargetArray _array_index (Math|Conversions|ToFloat(Integer) _array_element) true)))

(fn StringtoTransform
  (params (SourceString :type String))
  (LocalVariables|SetCSValueArray (Utilities|String|ParseIntoArray SourceString "," false))
  (return (Math|Transform|MakeTransform (Math|Vector|MakeVector (Math|Conversions|ToFloat(Integer) (Utilities|Array|Get(acopy) (LocalVariables|GetCSValueArray))) (Math|Conversions|ToFloat(Integer) (Utilities|Array|Get(acopy) (LocalVariables|GetCSValueArray) 1)) (Math|Conversions|ToFloat(Integer) (Utilities|Array|Get(acopy) (LocalVariables|GetCSValueArray) 2))) (Math|Rotator|MakeRotator (Math|Conversions|ToFloat(Integer) (Utilities|Array|Get(acopy) (LocalVariables|GetCSValueArray) 3)) (Math|Conversions|ToFloat(Integer) (Utilities|Array|Get(acopy) (LocalVariables|GetCSValueArray) 4)) (Math|Conversions|ToFloat(Integer) (Utilities|Array|Get(acopy) (LocalVariables|GetCSValueArray) 5))) (Math|Vector|MakeVector (Math|Conversions|ToFloat(Integer) (Utilities|Array|Get(acopy) (LocalVariables|GetCSValueArray) 6)) (Math|Conversions|ToFloat(Integer) (Utilities|Array|Get(acopy) (LocalVariables|GetCSValueArray) 7)) (Math|Conversions|ToFloat(Integer) (Utilities|Array|Get(acopy) (LocalVariables|GetCSValueArray) 8))))))

(fn UpdatePropertyonTargetObject
  (params (TargetObjectsArray :type Array%20of%20Object%20Object%20References) (NameOfThePropertyToUpdate :type Name) (DataToSet :type String))
  (LocalVariables|SetData%20to%20Set DataToSet)
  (LocalVariables|SetName%20Of%20the%20Property%20to%20Update NameOfThePropertyToUpdate)
  (LocalVariables|SetTarget%20Array TargetObjectsArray)
  (if (> (Utilities|Array|Length (LocalVariables|GetTarget%20Array)) 0)
    (for _array_element (LocalVariables|GetTarget%20Array)
      (Class|ExposeRuntimeFunctionsBPLibrary|SetFPropertybyName _array_element (LocalVariables|GetName%20Of%20the%20Property%20to%20Update) (LocalVariables|GetData%20to%20Set)))
    (else
      (Class|ExposeRuntimeFunctionsBPLibrary|SetFPropertybyName self (LocalVariables|GetName%20Of%20the%20Property%20to%20Update) (LocalVariables|GetData%20to%20Set)))))

(fn GetDefaultObject
  (params (TargetArray :type Array%20of%20Object%20Object%20References))
  (return (select (> (Utilities|Array|Length TargetArray) 0) (Utilities|Array|Get(acopy) TargetArray) self)))