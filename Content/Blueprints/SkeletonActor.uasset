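; SkeletonActor is a short-lived actor that animates its relative transform from a start to an end state, then destroys itself.
; The construction script builds the end transform from a forward distance, target rotation and end scale, with random sideways and vertical offsets from a time-seeded stream.
; On BeginPlay, a timeline with a randomized play rate around Speed drives the transform lerp and triggers destruction when finished.
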(event EventBeginPlay
  (bind _speed (Variables|Default|GetSpeed))
  (bind _speeddelta (Variables|Default|GetSpeedDelta))
  (Components|Timeline|SetPlayRate (Variables|Default|GetAnimationTimeline) (Math|Random|RandomFloatinRange (- _speed _speeddelta) (+ _speed _speeddelta)))
  (bind _alpha (Timeline|AnimationTimeline PlayFromStart)
    (:Update
      (Transformation|SetActorRelativeTransform (Math|Transform|Lerp(Transform) (Variables|Default|GetStartTransform) (Variables|Default|GetEndTransform) _alpha) false false))
    (:Finished
      ;[1 1 1] Destroy
      (Actor|DestroyActor))))

(fn ConstructionScript
  (Variables|Default|SetEndTransform (Math|Transform|MakeTransform (Math|Vector|MakeVector (Variables|Default|GetForwardDistance) (CallFunction|GetRandomFloat) (CallFunction|GetRandomFloat)) (Variables|Default|GetTargetRotation) (Variables|Default|GetEndScale))))

(fn GetRandomFloat
  (bind _deltalocation (Variables|Default|GetDeltaLocation))
  (return (Math|Random|RandomFloatinRangefromStream (* _deltalocation -1.0) _deltalocation (Math|Random|MakeRandomStream (* (.millisecond (Math|DateTime|Now)) (Math|Random|RandomInteger 33552))))))