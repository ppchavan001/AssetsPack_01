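; ParticleTransformComponent is a scene component that acts as a short-lived moving particle, carrying any attached child components.
; BeginPlay stores a start transform and a randomly offset end transform, though nothing in this graph applies either.
; Tick instead nudges relative location along the forward vector at a speed re-randomized every frame, keeping rotation and scale.
; After ParticleLifetime, it destroys all child components and then itself.
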(event EventTick
  (params (DeltaSeconds :type Float%20%28single-precision%29))
  (bind _speed (Variables|Default|GetSpeed))
  (bind _speeddelta (Variables|Default|GetSpeedDelta))
  (Transformation|SetRelativeTransform (Math|Transform|MakeTransform (+ (Variables|Default|GetRelativeLocation) (* (Math|Vector|GetForwardVector) (* DeltaSeconds (Math|Random|RandomFloatinRange (- _speed _speeddelta) (+ _speed _speeddelta))))) (Variables|Default|GetRelativeRotation) (Variables|Default|GetRelativeScale3D)) false false))

(event EventBeginPlay
  (bind _returnvalue (Transformation|GetRelativeTransform))
  (Utilities|FlowControl|Sequence
    (:then_0
      (Variables|Default|SetStartTransform (Math|Transform|MakeTransform (.location _returnvalue) (.rotation _returnvalue) (Variables|Default|GetStartScale)))
      (Variables|Default|SetEndTransform (Math|Transform|MakeTransform (+ (.location (Variables|Default|GetStartTransform)) (+ (* (Math|Vector|GetForwardVector) (Variables|Default|GetForwardDistance)) (* (Math|Vector|GetRightVector) (Math|Random|RandomFloatinRange (* (Variables|Default|GetRightDistanceMax) -1.0) (Variables|Default|GetRightDistanceMax))) (* (Math|Vector|GetUpVector) (Math|Random|RandomFloatinRange (* (Variables|Default|GetUpDistanceMax) -1.0) (Variables|Default|GetUpDistanceMax))))) (.rotation (Variables|Default|GetStartTransform)) (Variables|Default|GetEndScale))))
    (:then_1
      ;[1 1 1] Destroy
      (Utilities|FlowControl|Delay (Variables|Default|GetParticleLifetime))
      (for _array_element (Components|GetChildrenComponents true)
        (Components|DestroyComponent _array_element))
      (Components|DestroyComponent))))