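; Configurable LED wall actor that lays out a tile grid and exports it as a PFM file.
; BuildTileHierarchy clears old pieces, chains column scene components with per-column offset and rotation to curve the wall, then attaches spawned tiles down each.
; ExportPFM calls GeneratePFMEx relative to an optional origin, flagging fake tiles invalid; only the Z column angle is passed.
; ExportVerticesOnly writes GeneratePFMData vertices to Vertices.ini.
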(event Custom|Clean
  (CallFunction|DoClean))

(event Custom|ExportPFM
  (CallFunction|DoExportPFM))

(event Custom|BuildTileHierarchy
  (CallFunction|DoBuild))

(fn ConstructionScript
  (CallFunction|UpdateTexSize))

(fn DoClean
  (Utilities|FlowControl|Sequence
    (:then_0
      ;[1 1 1] Delete tiles
      (bind _outactors (Actor|GetAllActorsOfClass (Variables|TileSettings|GetTileType)))
      (bind _arrayelement (Utilities|Array|ReverseforEachLoop _outactors)
        (:LoopBody
          (if (== (Actor|GetAttachParentActor _arrayelement) self)
            (Actor|DestroyActor _arrayelement)))))
    (:then_1
      ;[1 1 1] Remove column markers
      (for _array_element (Variables|Internals|GetColumnComps)
        (Utilities|IsValid _array_element
          (:Is%20Valid
            (Components|DestroyComponent _array_element)))))
    (:then_2
      (Utilities|Array|Clear (Variables|Internals|GetTiles))
      (Utilities|Array|Clear (Variables|Internals|GetColumnComps)))))

(fn DoBuild
  (bind _columncomps (Variables|Internals|GetColumnComps))
  (CallFunction|UpdateTexSize)
  (Utilities|FlowControl|Sequence
    (:then_0
      ;[1 1 1] Clear previously generated stuff
      (CallFunction|Clean))
    (:then_1
      ;[1 1 1] Compute column base points
      (for _index (range 0 (Variables|Geometry|GetNb%20Columns))
        (LocalVariables|SetColIdx _index)
        (bind _returnvalue (AddComponent|AddSceneComponent false))
        (bind _output_get (Variables|Default|SetNewColumnRoot _returnvalue))
        (Transformation|AttachComponentToComponent _output_get (select (> (LocalVariables|GetColIdx) 0) (Utilities|Array|Get(acopy) (Variables|Internals|GetColumnComps) (- (LocalVariables|GetColIdx) 1)) (Variables|Default|GetDefaultSceneRoot)) "None" "KeepRelative" "KeepRelative" "KeepRelative" true)
        (Transformation|SetRelativeTransform (Variables|Default|GetNewColumnRoot) (select (> (LocalVariables|GetColIdx) 0) (Math|Transform|MakeTransform (Math|Vector|MakeVector 0.0 (Variables|TileSettings|GetTileWidth) 0.0) (Math|Rotator|MakeRotator (Variables|Geometry|GetAngle%20Between%20ColumnsX) (Variables|Geometry|GetAngle%20Between%20ColumnsY) (Variables|Geometry|GetAngle%20Between%20ColumnsZ))) (Math|Transform|MakeTransform "0, 0, 0")) false false)
        (bind _returnvalue_2 (Utilities|Array|Add (Variables|Internals|GetColumnComps) (Variables|Default|GetNewColumnRoot)))))
    (:then_2
      ;[1 1 1] Spawn tiles
      (for _index_2 (range 0 (- (Variables|Geometry|GetNb%20Columns) 1))
        (LocalVariables|SetColIdx _index_2)
        (for _index_3 (range 0 (- (Variables|Geometry|GetNb%20Rows) 1))
          (LocalVariables|SetRowIdx _index_3)
          (bind _returnvalue_3 (Game|SpawnActorfromClass (Variables|TileSettings|GetTileType) (Math|Transform|MakeTransform "0, 0, 0") "Undefined" 0 (Variables|TileSettings|GetTileWidth) (Variables|TileSettings|GetTileHeight) (Variables|TileSettings|GetTileWidthInPixels) (Variables|TileSettings|GetTileHeightInPixels) (LocalVariables|GetColIdx) (LocalVariables|GetRowIdx) (Utilities|Set|Contains (Variables|Geometry|GetFakeTileIndecies) (+ (LocalVariables|GetRowIdx) (* (LocalVariables|GetColIdx) (Variables|Geometry|GetNb%20Rows)))) (Variables|TileSettings|GetShow%20Tile%20ID) (Variables|TileSettings|GetTile%20IDScale) 0))
          (Utilities|Array|Add (Variables|Internals|GetTiles) _returnvalue_3)
          (Transformation|AttachComponentToComponent _returnvalue_3 (Utilities|Array|Get(acopy) (Variables|Internals|GetColumnComps) (LocalVariables|GetColIdx)) "None" "KeepRelative" "KeepRelative" "KeepRelative" true)
          (Transformation|SetActorRelativeLocation _returnvalue_3 (Math|Vector|MakeVector 0.0 0.0 (* (* (LocalVariables|GetRowIdx) (Variables|TileSettings|GetTileHeight)) -1.0))))))
    (:then_3
      (Development|PrintString (Utilities|String|Append "Placed " (Utilities|String|ToString(Integer) (Utilities|Array|Length (Variables|Internals|GetTiles))) " tiles."))
      (Development|PrintString (Utilities|String|Append "Wall left corner world location: " (Utilities|String|ToString(Vector) (Transformation|GetWorldLocation (Utilities|Array|Get(acopy) (Variables|Internals|GetColumnComps))))))
      (Development|PrintString (Utilities|String|Append "Wall right corner world location: " (Utilities|String|ToString(Vector) (Transformation|GetWorldLocation (Utilities|Array|Get(acopy) _columncomps (- (Utilities|Array|Length _columncomps) 1)))))))))

(fn DoExportPFM
  (bind _self self)
  (bind _path (Variables|PFM|GetPath))
  (bind _path_2 (Utilities|Struct|BreakDirectoryPath _path))
  (bind _returnvalue (Utilities|GetDisplayName _self))
  (bind _returnvalue_2 (Utilities|String|Append _path_2 "/" _returnvalue ".pfm"))
  (Utilities|FlowControl|Sequence
    (:then_0)
    (:then_1
      ;[1 1 1] Use self if no origin specified
      (LocalVariables|SetCurOrigin (select (Utilities|IsValid (Variables|PFM|GetOrigin)) (Variables|PFM|GetOrigin) self)))
    (:then_2
      ;[1 1 1] Clean temporary data
      (Utilities|Array|Clear (Variables|PFM|GetPFM%20Data))
      (Utilities|Array|Clear (Variables|PFM|GetPFM%20Data%20Validity)))
    (:then_3
      ;[1 1 1] Fill tiles validity array
      (if (> (Utilities|Array|Length (Variables|Internals|GetTiles)) 0)
        (for _array_element (Variables|Internals|GetTiles)
          (Utilities|Array|Add (Variables|PFM|GetPFM%20Data%20Validity) (not (Variables|/WarpUtils/LED/BP_LEDTile.BP_LEDTile_C|GetIsFakeTile _array_element))))
        (else
          (for _index (range 0 (- (* (Variables|Geometry|GetNb%20Columns) (Variables|Geometry|GetNb%20Rows)) 1))
            (Utilities|Array|Add (Variables|PFM|GetPFM%20Data%20Validity) true)))))
    (:then_4
      ;[1 1 1] Generate & save PFM
      (Development|PrintString _returnvalue_2)
      (bind _returnvalue_3 (Class|WarpUtilsBlueprintLibrary|GeneratePFMEx _returnvalue_2 (Transformation|GetActorLocation) (Transformation|GetActorRotation) (LocalVariables|GetCurOrigin) (Variables|Geometry|GetNb%20Columns) (Variables|Geometry|GetNb%20Rows) (Variables|Geometry|GetAngle%20Between%20ColumnsZ) (Variables|TileSettings|GetTileWidth) (Variables|TileSettings|GetTileHeight) (Variables|TileSettings|GetTileWidthInPixels) (Variables|TileSettings|GetTileHeightInPixels) (Variables|TileSettings|GetAddTileMargin) (Variables|PFM|GetPFM%20Data%20Validity)))
      (Development|PrintString (select _returnvalue_3 "PFM Export: OK" "PFM Export: FAILED") true true (select _returnvalue_3 "(R=0.068148,G=0.687500,B=0.046760,A=1.000000)" "(R=1.000000,G=0.027019,B=0.000000,A=1.000000)") 3.0))
    (:then_5
      ;[1 1 1] Clean temporary data
      (Utilities|Array|Clear (Variables|PFM|GetPFM%20Data))
      (Utilities|Array|Clear (Variables|PFM|GetPFM%20Data%20Validity)))))

(fn UpdateTexSize
  ;[1 1 1] Compute output texture size
  (Variables|PFM|SetTexture%20Width (* (Variables|Geometry|GetNb%20Columns) (Variables|TileSettings|GetTileWidthInPixels)))
  (Variables|PFM|SetTexture%20Height (* (Variables|Geometry|GetNb%20Rows) (Variables|TileSettings|GetTileHeightInPixels))))

(fn ExportVerticesOnly
  (bind _self self)
  (bind _path (Variables|PFM|GetPath))
  (bind _path_2 (Utilities|Struct|BreakDirectoryPath _path))
  (bind _returnvalue (Utilities|GetDisplayName _self))
  (bind _returnvalue_2 (Utilities|String|Append _path_2 "/" _returnvalue ".pfm"))
  (Utilities|FlowControl|Sequence
    (:then_0)
    (:then_1
      ;[1 1 1] Use self if no origin specified
      (LocalVariables|SetCurOrigin (select (Utilities|IsValid (Variables|PFM|GetOrigin)) (Variables|PFM|GetOrigin) self)))
    (:then_2
      ;[1 1 1] Clean temporary data
      (Utilities|Array|Clear (Variables|PFM|GetPFM%20Data))
      (Utilities|Array|Clear (Variables|PFM|GetPFM%20Data%20Validity)))
    (:then_3
      ;[1 1 1] Fill tiles validity array
      (if (> (Utilities|Array|Length (Variables|Internals|GetTiles)) 0)
        (for _array_element (Variables|Internals|GetTiles)
          (Utilities|Array|Add (Variables|PFM|GetPFM%20Data%20Validity) (not (Variables|/WarpUtils/LED/BP_LEDTile.BP_LEDTile_C|GetIsFakeTile _array_element))))
        (else
          (for _index (range 0 (- (* (Variables|Geometry|GetNb%20Columns) (Variables|Geometry|GetNb%20Rows)) 1))
            (Utilities|Array|Add (Variables|PFM|GetPFM%20Data%20Validity) true)))))
    (:then_4
      ;[1 1 1] Generate & save PFM
      (Development|PrintString _returnvalue_2)
      (bind _returnvalue_3 (Class|WarpUtilsBlueprintLibrary|GeneratePFMData _returnvalue_2 (Transformation|GetActorLocation) (Transformation|GetActorRotation) (LocalVariables|GetCurOrigin) (Variables|Geometry|GetNb%20Columns) (Variables|Geometry|GetNb%20Rows) (Variables|Geometry|GetAngle%20Between%20ColumnsZ) (Variables|TileSettings|GetTileWidth) (Variables|TileSettings|GetTileHeight) (Variables|TileSettings|GetTileWidthInPixels) (Variables|TileSettings|GetTileHeightInPixels) (Variables|TileSettings|GetAddTileMargin) (Variables|PFM|GetPFM%20Data%20Validity)))
      (bind _returnvalue_4 (Class|ExposeRuntimeFunctionsBPLibrary|ConvertVectorArraytoString _returnvalue_3))
      (Class|FileSDKBPLibrary|WriteStringtoFile (Utilities|String|Append (Class|BlueprintPathsLibrary|ProjectDir) "/Vertices.ini") _returnvalue_4 false "AutoDetect"))
    (:then_5
      ;[1 1 1] Clean temporary data
      (Utilities|Array|Clear (Variables|PFM|GetPFM%20Data))
      (Utilities|Array|Clear (Variables|PFM|GetPFM%20Data%20Validity)))))