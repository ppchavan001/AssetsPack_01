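; VertexManager is an actor that loads, adjusts and exports a vertex grid as a PFM file.
; BuildVertexData parses a text file into the Vertices array, which DeltaVertices offsets through AddDeltaToMatrixVertices using a maximum delta, matrix width and invert flag.
; ShowPoints batch-draws the points relative to the actor, and ExportPFM saves them to ExportedPFM.pfm in the project directory.
; Helper functions do the bulk work, leaving older Blueprint loops unconnected.
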(event Custom|DeltaVertices
  (bind _returnvalue (Class|ExposeRuntimeFunctionsBPLibrary|AddDeltatoMatrixVertices (Variables|Default|GetVertices) 2 (Variables|Default|GetMaxVertexDelta) (Variables|Default|GetMatrixWidth) (Variables|Default|GetInvertEffect)))
  (Variables|Default|SetVertices _returnvalue))

(event Custom|ExportPFM
  (bind _returnvalue (Class|WarpUtilsBlueprintLibrary|SavePFM (Utilities|String|Append (Class|KismetSystemLibrary|GetProjectDirectory) "/ExportedPFM.pfm") (Variables|Default|GetMatrixWidth) (Variables|Default|GetMatrixHeight) (Variables|Default|GetVertices)))
  (Development|PrintString (Utilities|String|Append "PFM Exported: " (Utilities|String|ToString(Boolean) _returnvalue))))

(event Custom|ShowPoints
  (Class|ExposeRuntimeFunctionsBPLibrary|MassDebugDrawPoint (Variables|Default|GetVertices) (Transformation|GetActorLocation) self 1.0 (Math|Conversions|ToColor(LinearColor) "(R=0.857144,G=1.000000,B=0.000000,A=1.000000)") false 5.0))

(fn ConstructionScript)

(fn BuildVertexData
  (bind _verticesout (Class|ExposeRuntimeFunctionsBPLibrary|ConvertStringtoVector (.Lines (Class|FileSDKBPLibrary|ReadLinesfromFile (Utilities|Struct|BreakFilePath (Variables|Default|GetVertexFile))))))
  (Variables|Default|SetVertices _verticesout))